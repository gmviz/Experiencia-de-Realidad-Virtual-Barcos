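; BP_Cannon is a VR cannon that the player aims by grabbing and fires by lighting with a torch.
; While grabbed, the motion controller's world Y offset drives the barrel's yaw within a clamped arc.
; When not grabbed, Tick checks BP_Antorcha's proximity to the fuse sphere, starting effects, then a delayed spawn at the arrow with haptics and sound.
; A hint light appears if the cannon stays unfired after BeginPlay.
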(event OnGrabbed(BP_GrabComponent)
  (Variables|Default|SetInitialHandY (.y (Transformation|GetWorldLocation (Actor|GetComponentbyClass (Game|Player|GetPlayerPawn 0) "/Script/HeadMountedDisplay.MotionControllerComponent"))))
  (Variables|Default|SetInitialCannonYaw (.yaw (Variables|/Script/Engine.SceneComponent|GetRelativeRotation (Variables|Default|GetCanon))))
  (Variables|Default|SetbIsAiming true))

(event OnDropped(BP_GrabComponent)
  (Variables|Default|SetbIsAiming false))

(event EventBeginPlay
  (Utilities|FlowControl|Delay 15.0)
  (if (not (Variables|Default|GetbHaDisparado))
    (Rendering|SetVisibility (Variables|Default|GetPointLight) true false)))

(event Collision|EventActorBeginOverlap
  (params (OtherActor :type Actor%20Object%20Reference)))

(event EventTick
  (params (DeltaSeconds :type Float%20%28single-precision%29))
  (if (Variables|Default|GetbIsAiming)
    (Transformation|SetRelativeRotation (Variables|Default|GetCanon) (Math|Rotator|MakeRotator 0.0 0.0 (Math|Float|ClampAngle (+ (* (- (.y (Transformation|GetWorldLocation (Actor|GetComponentbyClass (Game|Player|GetPlayerPawn 0) "/Script/HeadMountedDisplay.MotionControllerComponent"))) (Variables|Default|GetInitialHandY)) 1.5) (Variables|Default|GetInitialCannonYaw)) -45.0 45.0)) false false)
    (else
      (bind _returnvalue (Actor|GetActorOfClass "/Game/Antorcha/BP_Antorcha.BP_Antorcha_C"))
      (if (and (< (Math|Vector|Distance(Vector) (Transformation|GetWorldLocation (Variables|Default|GetSphere)) (Transformation|GetActorLocation _returnvalue)) 5e+01) (not (Variables|Default|GetbIsFuseLit)))
        (Variables|Default|SetbIsFuseLit true)
        (Variables|Default|SetbHaDisparado true)
        (Rendering|SetVisibility (Variables|Default|GetPointLight) false false)
        (Components|Activation|Activate (Variables|Default|GetNiagara) false)
        (Audio|Components|Audio|Play (Variables|Default|GetAudioMecha) 0.0)
        (Utilities|FlowControl|Delay 4.5)
        (Game|SpawnActorfromClass "/Game/Cannon/BP_Projectile.BP_Projectile_C" (Transformation|GetWorldTransform (Variables|Default|GetArrow)) "AlwaysSpawn" "MultiplyWithRoot" self 0)
        (Class|PlayerController|PlayHapticEffect (Game|GetPlayerController 0) "/Game/XRFramework/Haptics/PistolFireHapticEffect.PistolFireHapticEffect" "Right" 2.0 false)
        (Class|PlayerController|PlayHapticEffect (Game|GetPlayerController 0) "/Game/XRFramework/Haptics/PistolFireHapticEffect.PistolFireHapticEffect" "Left" 2.0 false)
        (Audio|PlaySoundatLocation "/Game/Cannon/SFX_Cannon.SFX_Cannon" (Transformation|GetWorldLocation (Variables|Default|GetArrow)) "0, 0, 0" 1.0 1.0 0.0 0 0 0 0)
        (Components|Activation|Deactivate (Variables|Default|GetNiagara))
        (Variables|Default|SetbIsFuseLit false)))))

(fn ConstructionScript)