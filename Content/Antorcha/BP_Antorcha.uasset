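; Grabbable torch actor that returns to its starting transform after being dropped or falling out of the level.
; If it has not been grabbed shortly after BeginPlay, a point light turns on, and grabbing it turns that light off.
; Dropping it through BP_GrabComponent enables physics.
; A delayed response to any mesh hit, or a Tick height check, teleports it back and disables physics.
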(event OnComponentHit(Antorcha)
  (params (HitComponent :type Primitive%20Component%20Object%20Reference) (OtherActor :type Actor%20Object%20Reference) (OtherComp :type Primitive%20Component%20Object%20Reference) (NormalImpulse :type Vector :default "0, 0, 0") (Hit :type Hit%20Result%20Structure%20%28by%20ref%29))
  (Utilities|FlowControl|Delay 2.0)
  (Transformation|SetActorTransform (Variables|Default|GetPosicionInicial) false true)
  (Physics|SetPhysicsLinearVelocity (Variables|Default|GetAntorcha) "0, 0, 0" false "None")
  (Physics|SetSimulatePhysics (Variables|Default|GetAntorcha) false))

(event OnGrabbed(BP_GrabComponent)
  (Variables|Default|SetbAntorchaAgarrada true)
  (Rendering|SetVisibility (Variables|Default|GetPointLight) false false))

(event OnDropped(BP_GrabComponent)
  (Physics|SetSimulatePhysics (Variables|Default|GetAntorcha) true))

(event EventBeginPlay
  (Variables|Default|SetPosicionInicial (Transformation|GetActorTransform))
  (Utilities|FlowControl|Delay 15.0)
  (if (not (Variables|Default|GetbAntorchaAgarrada))
    (Rendering|SetVisibility (Variables|Default|GetPointLight) true false)))

(event EventTick
  (params (DeltaSeconds :type Float%20%28single-precision%29))
  (if (< (.z (Transformation|GetActorLocation)) -1e+02)
    (Transformation|SetActorTransform (Variables|Default|GetPosicionInicial) false true)
    (Physics|SetPhysicsLinearVelocity (Variables|Default|GetAntorcha) "0, 0, 0" false "None")
    (Physics|SetSimulatePhysics (Variables|Default|GetAntorcha) false)))

(fn ConstructionScript)